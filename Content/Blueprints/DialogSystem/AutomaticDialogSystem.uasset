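; Automatic dialogue Blueprint that plays a timed NPC conversation when its box trigger is first overlapped.
; On BeginPlay it caches text and speaker names from Dialogues table rows matching its NPCID and ConversationID.
; A looping timer advances the lines in a WBP_Dialogue widget, added through the player controller's HUDWidget.
; CreateDialog disables player movement on opening, then restores walking and removes the widget after the last line.
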(event `self.ReceiveBeginPlay`
  ;[0.1961 0.2124 1] Get all the lines for this character from the dialogue table
  (bind _outrownames (`DataTableFunctionLibrary.GetDataTableRowNames` "/Game/Blueprints/DialogSystem/Dialogues.Dialogues"))
  (for _array_element _outrownames
    (bind _returnvalue (`|GetDataTableRow` "/Game/Blueprints/DialogSystem/Dialogues.Dialogues" _array_element)
      (:`then`
        (bind (_npc_id _conversation_id _line_id _character_name _text) (break `/Game/Blueprints/DialogSystem/F_DialogueStructure` _returnvalue))
        (if (and (== _npc_id (`self.NPC_ID`)) (== _conversation_id (`self.Conversation_ID`)))
          (`KismetArrayLibrary.Array_Add` (`self.AutomaticDialogue`) _text)
          (`KismetArrayLibrary.Array_Add` (`self.DialogueCharacterName`) _character_name))))))

(event `StartConversation`
  (params (TimeBetweenLines :type "Float (double-precision)"))
  ;[0.1531 1 0.1804] Player starts the conversation
  (`self.GetLineAndShow`)
  (bind _returnvalue (`KismetSystemLibrary.K2_SetTimerDelegate` (delegate `GetLineAndShow`) TimeBetweenLines true))
  (set `self.DialogueTimer` _returnvalue))

(event `GetLineAndShow`
  (bind _returnvalue (> (`KismetArrayLibrary.Array_Length` (`self.AutomaticDialogue`)) (`self.CurrentLine`)))
  (`self.CreateDialog` (not _returnvalue))
  ;[1 0.3521 0.1511] Set the next line of the dialog and change the character name
  (if _returnvalue
    (`TextBlock.SetText` (`/Game/Blueprints/DialogSystem/Wdigets/WBP_Dialogue.DialogueText` (`self.Dialogue Widget`)) (`|GetArrayItem` (`self.AutomaticDialogue`) (`self.CurrentLine`)))
    (`/Game/Blueprints/DialogSystem/Wdigets/WBP_Dialogue.ChangeCharacterName` (`self.Dialogue Widget`) (`|GetArrayItem` (`self.DialogueCharacterName`) (`self.CurrentLine`)))
    (`/Engine/EditorBlueprintResources/StandardMacros.IncrementInt` (`self.CurrentLine`))
    (else
      (`KismetSystemLibrary.K2_ClearAndInvalidateTimerHandle` (`self.DialogueTimer`))
      (set `self.CurrentLine` 0))))

(event `self.Box.OnComponentBeginOverlap`
  (params (OverlappedComponent :type "PrimitiveComponent Object Reference") (OtherActor :type "Actor Object Reference") (OtherComp :type "PrimitiveComponent Object Reference") (OtherBodyIndex :type Integer) (bFromSweep :type Boolean) (SweepResult :type "HitResult Structure (by ref)"))
  ;[1 1 1] Just a test when the player overlaps a collider
  (if (`self.CanStartConversation?`)
    (`self.StartConversation` 2.0)
    (set `self.CanStartConversation?` false)))

(fn `CreateDialog`
  (params (`CloseDialog?` :type Boolean))
  (`self.Dialogue Widget`
    (:`then`
      (if `CloseDialog?`
        ;[1 0.257 0.08683] Enable Character movement and remove Widget
        (`CharacterMovementComponent.SetMovementMode` (`Character.CharacterMovement` (`GameplayStatics.GetPlayerCharacter` 0)) "MOVE_Walking" 0)
        (`Widget.RemoveFromParent` (`self.Dialogue Widget`))
        (set `self.Dialogue Widget` null)))
    (:`else`
      ;[0.6766 0.3333 1] If there is no Dialog Widget Created: We create one and get the first line of the conversation and set the this character as the NPC for the HUDWidget
      (bind _returnvalue (`|CreateWidget` "/Game/Blueprints/DialogSystem/Wdigets/WBP_Dialogue.WBP_Dialogue_C" null "Test"))
      (set `self.Dialogue Widget` _returnvalue)
      (bind _aspcont (cast `/Game/Blueprints/TemporalCharacter/PCont` (`GameplayStatics.GetPlayerController` 0)))
      (`/Game/Blueprints/InventorySystem/Widgets/WBP_HUD.AddDialogueText` (`/Game/Blueprints/TemporalCharacter/PCont.HUDWidget` _aspcont) (`self.Dialogue Widget`))
      ;[0.3277 1 0.2491] Disable character movement
      (`CharacterMovementComponent.DisableMovement` (`Character.CharacterMovement` (`GameplayStatics.GetPlayerCharacter` 0))))))

(fn `UserConstructionScript`)