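; LightSwitch is a trigger-driven actor that fades a set of room lights in when the player enters and out when the player leaves.
; Overlap events on its Trigger, filtered to the first player's character, play a LightsOn timeline forward or a separate LightsOff timeline in reverse from the end.
; Each timeline update lerps every RoomLights entry's intensity between zero and its matching value in the parallel LightIntensities array.
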(event `self.Trigger.OnComponentBeginOverlap`
  (params (OverlappedComponent :type "PrimitiveComponent Object Reference") (OtherActor :type "Actor Object Reference") (OtherComp :type "PrimitiveComponent Object Reference") (OtherBodyIndex :type Integer) (bFromSweep :type Boolean) (SweepResult :type "HitResult Structure (by ref)"))
  (if (== OtherActor (`GameplayStatics.GetPlayerCharacter` 0))
    (bind (_direction _lighton) (`Timeline|LightsOn` :!via `PlayFromStart`)
      (:`Update`
        (for (_array_element _array_index) (`self.RoomLights`)
          (`LightComponent.SetIntensity` (`Light.LightComponent` _array_element) (`KismetMathLibrary.Lerp` 0.0 (`|GetArrayItem` (`self.LightIntensities`) _array_index) _lighton)))))))

(event `self.Trigger.OnComponentEndOverlap`
  (params (OverlappedComponent :type "PrimitiveComponent Object Reference") (OtherActor :type "Actor Object Reference") (OtherComp :type "PrimitiveComponent Object Reference") (OtherBodyIndex :type Integer))
  (if (== OtherActor (`GameplayStatics.GetPlayerCharacter` 0))
    (bind (_direction _lightoff) (`Timeline|LightsOff` :!via `ReverseFromEnd`)
      (:`Update`
        (for (_array_element _array_index) (`self.RoomLights`)
          (`LightComponent.SetIntensity` (`Light.LightComponent` _array_element) (`KismetMathLibrary.Lerp` 0.0 (`|GetArrayItem` (`self.LightIntensities`) _array_index) _lightoff)))))))

(fn `UserConstructionScript`)