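; NPC that roams to random nearby points and holds branching, data-table-driven conversations with the player.
; On BeginPlay it caches Dialogue rows matching its NPCID; each interaction advances the line and finds its text by conversation and line ID.
; Text appears in a dialogue widget on the player's HUD, with question answers jumping to their next line.
; Player movement is locked and the cursor shown until no line remains.
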(event `self.ReceiveBeginPlay`
  ;[0.1961 0.2124 1] Get all the lines for this character from the dialogue table
  (bind _outrownames (`DataTableFunctionLibrary.GetDataTableRowNames` "/Game/Blueprints/DialogSystem/Dialogue.Dialogue"))
  (for _array_element _outrownames
    (bind _returnvalue (`|GetDataTableRow` "/Game/Blueprints/DialogSystem/Dialogue.Dialogue" _array_element)
      (:`then`
        (if (== (`.NPC_ID_2_EE1BFD3B4868D3F40103E49A4B898EE7` (break `/Game/Blueprints/DialogSystem/F_DialogueStructure` _returnvalue)) (`self.NPC_ID`))
          (`KismetArrayLibrary.Array_Add` (`self.CharacterDialogue`) _array_element))))))

(event `/Game/Blueprints/BI_Interaction.Interaction`
  (params (Actor :type "Actor Object Reference"))
  ;[1 1 1] Player starts the conversation
  (set `self.IsTalking?` true)
  (`/Engine/EditorBlueprintResources/StandardMacros.IncrementInt` (`self.CurrentLine`)
    (:`  `
      (`self.Create Dialogue`))))

(event `self.ReceiveTick`
  (params (DeltaSeconds :type "Float (single-precision)"))
  ;[1 1 1] NPC Roaming
  (if (not (`self.IsTalking?`))
    (`KismetSystemLibrary.Delay` (`KismetMathLibrary.RandomFloatInRange` 5.0 15.0))
    (set `self.IsMoving?` true)
    (`|AIMoveTo` self (`NavigationSystemV1.K2_GetRandomReachablePointInRadius` (`self.K2_GetActorLocation`) 500.0 null null) null
      (:`OnSuccess`
        _)
      (:`OnFail`
        _))
    (set `self.IsMoving?` false)))

(fn `AnswerSelected`
  (params (NextLineID :type Integer))
  (set `self.CurrentLine` NextLineID)
  (set `self.CharacterAnswering` false)
  (`self.Dialogue Get Line And Update Text`))

(fn `Create Dialogue`
  (bind _returnvalue (`GameplayStatics.GetPlayerController` 0))
  (bind _returnvalue_2 (`GameplayStatics.GetPlayerController` 0))
  (if (not (`self.CharacterAnswering`))
    (`self.DialogueWidget`
      (:`then`
        _)
      (:`else`
        ;[0.6766 0.3333 1] If there is no Dialog Widget Created: We create one and get the first line of the conversation and set the this character as the NPC for the HUDWidget
        (bind _returnvalue_3 (`|CreateWidget` "/Game/Blueprints/DialogSystem/Wdigets/WBP_Dialogue.WBP_Dialogue_C" null (`self.CharacterName`)))
        (set `self.DialogueWidget` _returnvalue_3)
        (bind _aspcont (cast `/Game/Blueprints/TemporalCharacter/PCont` (`GameplayStatics.GetPlayerController` 0)))
        (bind _hudwidget (`/Game/Blueprints/TemporalCharacter/PCont.HUDWidget` _aspcont))
        (set `/Game/Blueprints/InventorySystem/Widgets/WBP_HUD.NPC` self _hudwidget)
        (`/Game/Blueprints/InventorySystem/Widgets/WBP_HUD.AddDialogueText` _hudwidget (`self.DialogueWidget`))))
    (bind _closewidget_ (`self.Dialogue Get Line And Update Text`))
    (if _closewidget_
      ;[1 0.257 0.08683] Enable Character movement
      (`CharacterMovementComponent.SetMovementMode` (`Character.CharacterMovement` (`GameplayStatics.GetPlayerCharacter` 0)) "MOVE_Walking" 0)
      (`WidgetBlueprintLibrary.SetInputMode_GameOnly` _returnvalue)
      (set `PlayerController.bShowMouseCursor` false _returnvalue)
      (else
        ;[0.3277 1 0.2491] Disable character movement and allow to use the mouse in the HUD
        (`CharacterMovementComponent.DisableMovement` (`Character.CharacterMovement` (`GameplayStatics.GetPlayerCharacter` 0)))
        (bind _aspcont_2 (cast `/Game/Blueprints/TemporalCharacter/PCont` _returnvalue_2))
        (`WidgetBlueprintLibrary.SetInputMode_GameAndUIEx` _returnvalue_2 (`/Game/Blueprints/TemporalCharacter/PCont.HUDWidget` _aspcont_2) "LockAlways")
        (set `PlayerController.bShowMouseCursor` true _returnvalue_2)))))

(fn `Dialogue Get Line And Update Text`
  (returns (`CloseWidget?` :type Boolean))
  (locals (ReturnedLines :type "Array of Text") (AnswerStructure :type "Array of /Game/Blueprints/DialogSystem/F_Answer Structure"))
  (for _array_element (`self.CharacterDialogue`)
    (bind _returnvalue (`|GetDataTableRow` "/Game/Blueprints/DialogSystem/Dialogue.Dialogue" _array_element)
      (:`then`
        (bind (_npc_id _conversation_id _line_id _text _question_ _answer_id _answer_text _next_line_id) (break `/Game/Blueprints/DialogSystem/F_DialogueStructure` _returnvalue))
        ;[1 0.3342 0.1435] If anything with the conversation ID and CurrentLine
        (if (and (== _conversation_id (`self.Conversation_ID`)) (== _line_id (`self.CurrentLine`)))
          ;[0.3374 1 0.2026] If Question, add all the answers, if not then just return the lines
          (if _question_
            (`KismetArrayLibrary.Array_Add` (`local.AnswerStructure`) (make `/Game/Blueprints/DialogSystem/F_Answer` _answer_text _next_line_id)))
          (`KismetArrayLibrary.Array_Add` (`local.ReturnedLines`) _text)))))
  ;[1 0.9432 0.1217] If line found, set the text and answers, if not delete it
  (if (> (`KismetArrayLibrary.Array_Length` (`local.ReturnedLines`)) 0)
    (`TextBlock.SetText` (`/Game/Blueprints/DialogSystem/Wdigets/WBP_Dialogue.DialogueText` (`self.DialogueWidget`)) (`|GetArrayItem` (`local.ReturnedLines`)))
    (`self.GetAnswers` (`local.AnswerStructure`))
    (return false)
    (else
      (`Widget.RemoveFromParent` (`self.DialogueWidget`))
      (set `self.DialogueWidget` null)
      (set `self.CurrentLine` 0)
      (return true))))

(fn `GetAnswers`
  (params (Answers :type "Array of /Game/Blueprints/DialogSystem/F_Answer Structure"))
  ;[0.2709 1 0.1983] Get the text of each answer and call a function of the HUDWidget to show it in the HUD
  (for _array_element Answers
    (bind _aspcont (cast `/Game/Blueprints/TemporalCharacter/PCont` (`GameplayStatics.GetPlayerController` 0)))
    (bind (_answer _nextlineid) (break `/Game/Blueprints/DialogSystem/F_Answer` _array_element))
    (`/Game/Blueprints/InventorySystem/Widgets/WBP_HUD.AddAnswers` (`/Game/Blueprints/TemporalCharacter/PCont.HUDWidget` _aspcont) _answer _nextlineid) ; Answer text and the next line id depending on the answer
    (set `self.CharacterAnswering` true)))

(fn `UserConstructionScript`)