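; Interactable bookshelf that opens a secret passage when the player uses it.
; It extends an interactable parent, adding a flavor message to its information array on BeginPlay.
; When the BookshelfInteraction flag is set, interaction runs the parent logic, then hides the referenced FakeWall actor, disables its collision and records BookshelfUsed on the GameInstance.
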(event `self.ReceiveBeginPlay`
  (`parent.ReceiveBeginPlay`)
  (`KismetArrayLibrary.Array_Add` (`self.ObjectInformationArray`) "You tried to move a book and something happened."))

(event `/Game/Blueprints/BI_Interaction.Interaction`
  (params (Actor :type "Actor Object Reference"))
  (if (`self.BookshelfInteraction`)
    (`parent.Interaction` Actor)
    (`self.HideFakeWall`)))

(fn `HideFakeWall`
  (bind _fakewall (`self.FakeWall`))
  (`self.SetActorHiddenInGame` _fakewall true)
  (`self.SetActorEnableCollision` _fakewall false)
  (bind _asgame_instance (cast `/Game/Blueprints/GameInstance` (`GameplayStatics.GetGameInstance`)))
  (set `/Game/Blueprints/GameInstance.BookshelfUsed` true _asgame_instance))

(fn `UserConstructionScript`
  (`parent.UserConstructionScript`))