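; B_InteractableObject is an interactable actor that shows informational text about itself on the player's HUD.
; Each Interaction call runs NextObjectLine, which swaps the HUD text widget for the next entry in ObjectInformationArray and disables player movement.
; After the last line, the following interaction removes the text, restores walking, resets the index and sets FinishInteraction.
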(event `self.ReceiveActorBeginOverlap`
  (params (OtherActor :type "Actor Object Reference")))

(event `/Game/Blueprints/BI_Interaction.Interaction`
  (params (Actor :type "Actor Object Reference"))
  (if (`self.CanCloseDialog?`)
    ;[1 0.9764 0.1674] Removes the text from the HUD and the player can move again
    (set `self.CanCloseDialog?` false)
    (bind _aspcont (cast `/Game/Blueprints/TemporalCharacter/PCont` (`GameplayStatics.GetPlayerController` 0)))
    (`/Game/Blueprints/InventorySystem/Widgets/WBP_HUD.RemoveTextFromHUD` (`/Game/Blueprints/TemporalCharacter/PCont.HUDWidget` _aspcont) (`self.Text Information Widget`))
    (`CharacterMovementComponent.SetMovementMode` (`Character.CharacterMovement` (`GameplayStatics.GetPlayerCharacter` 0)) "MOVE_Walking" 0)
    (set `self.ObjectInformationID` 0)
    (set `self.FinishInteraction` true)
    (else
      (set `self.FinishInteraction` false)
      (`self.NextObjectLine`))))

(fn `NextObjectLine`
  ;[0.2754 0.2314 1] Show in the HUD a text about the object, and the player cannot move
  (if (> (`KismetArrayLibrary.Array_Length` (`self.ObjectInformationArray`)) (`self.ObjectInformationID`))
    (bind _aspcont (cast `/Game/Blueprints/TemporalCharacter/PCont` (`GameplayStatics.GetPlayerController` 0)))
    (bind _hudwidget (`/Game/Blueprints/TemporalCharacter/PCont.HUDWidget` _aspcont))
    (`/Game/Blueprints/InventorySystem/Widgets/WBP_HUD.RemoveTextFromHUD` _hudwidget (`self.Text Information Widget`))
    (bind _textinformationwidget (`/Game/Blueprints/InventorySystem/Widgets/WBP_HUD.AddInformationTextOfObjectToHUD` _hudwidget (`|GetArrayItem` (`self.ObjectInformationArray`) (`self.ObjectInformationID`))))
    (set `self.Text Information Widget` _textinformationwidget)
    (`CharacterMovementComponent.DisableMovement` (`Character.CharacterMovement` (`GameplayStatics.GetPlayerCharacter` 0)))
    (set `self.ObjectInformationID` (+ (`self.ObjectInformationID`) 1))
    (if (<= (`KismetArrayLibrary.Array_Length` (`self.ObjectInformationArray`)) (`self.ObjectInformationID`))
      (set `self.CanCloseDialog?` true))))

(fn `UserConstructionScript`)