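; Interactable bed drawer that slides open and lets the player place a jug in it.
; During the first-time phase, interaction plays a timeline that lerps the drawer open, until CanCloseDialog ends that phase.
; Later interactions scan the player's inventory component for the jug by name and swap in its info text.
; With the jug found and FinishInteraction unset, a DoOnce spawns it at the drawer and clears the text.
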(event `self.ReceiveActorBeginOverlap`
  (params (OtherActor :type "Actor Object Reference"))
  (`parent.ReceiveActorBeginOverlap` OtherActor))

(event `/Game/Blueprints/BI_Interaction.Interaction`
  (params (Actor :type "Actor Object Reference"))
  (`parent.Interaction` Actor)
  (if (`self.FirstTimeInteraction`)
    (if (`self.CanCloseDialog?`)
      (set `self.FirstTimeInteraction` false)
      (else
        ;[1 0.9369 0.1534] Open drawer and check if Jug is in the inventory
        (bind (_direction _movedrawer) (`Timeline|MoveDrawer`)
          (:`Update`
            (`SceneComponent.K2_SetRelativeLocation` (`self.SM_Bed_Drawer_Openable_Part`) (`KismetMathLibrary.VLerp` (`KismetMathLibrary.MakeVector` 0.0 10.0) (`KismetMathLibrary.MakeVector` 0.0 45.0) _movedrawer) false false)))))
    (elif (and (`self.JugInInventory`) (not (`self.FinishInteraction`)))
      (`/Engine/EditorBlueprintResources/StandardMacros.DoOnce` false
        (:`Completed`
          ;[1 0.1813 0.1116] Place Jug in the drawer
          (`|SpawnActorFromClass` "/Game/Blueprints/Puzzles/Jugs/Jug.Jug_C" (`KismetMathLibrary.MakeTransform` (+ (`SceneComponent.K2_GetComponentLocation` (`self.SM_Bed_Drawer_Openable_Part`)) (-20.0 0.0 80.0)) (struct :`Yaw` -90.0)) "Undefined" "OverrideRootScale" null null null)
          (`KismetArrayLibrary.Array_Clear` (`self.ObjectInformationArray`))))
      (else
        (`/Engine/EditorBlueprintResources/StandardMacros.DoOnce` false
          (:`Completed`
            (`self.CheckIfJugInInventory`)))))))

(fn `CheckIfJugInInventory`
  (bind _objectinformationarray (`self.ObjectInformationArray`))
  (bind _asplayer_character (cast `/Game/Blueprints/PlayerController/PlayerCharacter` (`GameplayStatics.GetPlayerCharacter` 0)))
  ;[0.4124 1 0.2487] Check the player inventory and set variable if the jug is in the inventory
  (for _array_element (`/Game/Blueprints/InventorySystem/PickableObjects/AC_Inventory.Inventory` (`/Game/Blueprints/PlayerController/PlayerCharacter.AC_Inventory` _asplayer_character))
    (if (`KismetTextLibrary.EqualEqual_TextText` (`.Name_2_B3B5A6A145432A9B2505B5AE2F9FFDB6` (break `/Game/Blueprints/InventorySystem/PickableObjects/F_Object` (`.ObjectStructure_2_89C0947C4FA810AB2C118F9E115F387F` (break `/Game/Blueprints/InventorySystem/PickableObjects/F_Slot` _array_element)))) (`self.JugName`))
      (set `self.JugInInventory` true)
      (`KismetArrayLibrary.Array_Clear` _objectinformationarray)
      (`KismetArrayLibrary.Array_Add` _objectinformationarray (`self.TextAboutJug`))
      (break))))

(fn `UserConstructionScript`
  (`parent.UserConstructionScript`))