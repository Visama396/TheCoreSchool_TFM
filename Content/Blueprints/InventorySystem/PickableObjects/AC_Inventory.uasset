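; Inventory component that stores items in a fixed-size slot array and toggles the player's inventory window.
; Stackable items add one to a same-class stack below its max, while others, or those without such a stack, take the slot matching an empty "Nothing" placeholder.
; Toggling adds WBP_Inventory to the HUD canvas and disables movement, or removes it, restores walking and game input, and destroys any spawned object.
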(event `self.ReceiveBeginPlay`
  (`self.InitInventory`))

(fn `Add to Inventory`
  (params (ContentToAdd :type "/Game/Blueprints/InventorySystem/PickableObjects/F_Slot Structure"))
  (returns (`Added?` :type Boolean))
  ;[1 0.28 0.3199] If the item is not stackable
  (if (`.IsStackable_6_09476A8740EE494AFB585CBB8FCD624C` (break `/Game/Blueprints/InventorySystem/PickableObjects/F_Object` (break `/Game/Blueprints/InventorySystem/PickableObjects/F_Slot` ContentToAdd)))
    (`self.AddToStack` (`local.ContentToAdd`))
    (else
      (`self.CreateStack` (`local.ContentToAdd`))))
  (return true))

(fn `AddToStack`
  (params (ContentToAdd :type "/Game/Blueprints/InventorySystem/PickableObjects/F_Slot Structure"))
  (set `self.ObjectAdded` false)
  ;[0.358 1 0.1384] First check if in the inventory, there is any object with the same name, and the ammount of objects is not bigger than the MaxStack
  (for (_array_element _array_index) (`self.Inventory`)
    (bind (_objectstructure _ammount) (break `/Game/Blueprints/InventorySystem/PickableObjects/F_Slot` _array_element))
    (if (== (`.Class_15_DB5D15A14E9C71F7312C2E8A14BC0C2B` (break `/Game/Blueprints/InventorySystem/PickableObjects/F_Object` _objectstructure)) (`.Class_15_DB5D15A14E9C71F7312C2E8A14BC0C2B` (break `/Game/Blueprints/InventorySystem/PickableObjects/F_Object` (`.ObjectStructure_2_89C0947C4FA810AB2C118F9E115F387F` (break `/Game/Blueprints/InventorySystem/PickableObjects/F_Slot` ContentToAdd)))))
      (if (< _ammount (`.MaxStack_12_FC0CC1ED4F33DC5444504E9F977A40C1` (break `/Game/Blueprints/InventorySystem/PickableObjects/F_Object` _objectstructure)))
        ;[0.3501 0.2964 1] Add 1 to the ammount of objects of this type
        (bind _structout (setmembers `/Game/Blueprints/InventorySystem/PickableObjects/F_Slot` :`StructRef` _array_element :`Ammount` (+ (`.Ammount_5_EF391DE04DBEF3DBCF4882B8D9F790F1` (break `/Game/Blueprints/InventorySystem/PickableObjects/F_Slot` _array_element)) 1)))
        (`KismetArrayLibrary.Array_Set` (`self.Inventory`) _array_index _structout)
        (set `self.ObjectAdded` true)
        (break))))
  ;[1 0.2028 0.2925] If no object was added, add a new Stack with ammount 1
  (if (not (`self.ObjectAdded`))
    (`self.CreateStack` ContentToAdd)
    (set `self.ObjectAdded` true)))

(fn `CreateStack`
  (params (ContentToAdd :type "/Game/Blueprints/InventorySystem/PickableObjects/F_Slot Structure"))
  (bind _inventory (`self.Inventory`))
  ;[0.6046 0.2291 1] Searches in the inventory the slot with ammount 0 and adds in that position a new slot for the new item
  (`KismetArrayLibrary.Array_Set` _inventory (`KismetArrayLibrary.Array_Find` _inventory (make `/Game/Blueprints/InventorySystem/PickableObjects/F_Slot` (make `/Game/Blueprints/InventorySystem/PickableObjects/F_Object` "Nothing" false null 5 "/Game/Blueprints/InventorySystem/PickableObjects/B_PickableObject.B_PickableObject_C"))) ContentToAdd))

(fn `InitInventory`
  (`KismetArrayLibrary.Array_Resize` (`self.Inventory`) (`self.Slots`)))

(fn `OpenCloseInventory`
  (bind _inventorywindow (`self.InventoryWindow`))
  (bind _spawnedobject (`self.SpawnedObject`))
  (bind _inventorywindow_2 (`self.InventoryWindow`)
    (:`then`
      (`Widget.RemoveFromParent` _inventorywindow_2)
      (set `self.InventoryWindow` null)
      (`WidgetBlueprintLibrary.SetInputMode_GameOnly` (`GameplayStatics.GetPlayerController` 0))
      (`CharacterMovementComponent.SetMovementMode` (`Character.CharacterMovement` (`GameplayStatics.GetPlayerCharacter` 0)) "MOVE_Walking" 0)
      (`/Engine/EditorBlueprintResources/StandardMacros.IsValid` _spawnedobject
        (:`Is Valid`
          (`Actor.K2_DestroyActor` _spawnedobject) ; Destroy Spawned Object
        )))
    (:`else`
      ;[0.4536 1 0.3115] If does not exist, create inventory widget and save it as variable
      (bind _returnvalue (`|CreateWidget` "/Game/Blueprints/InventorySystem/Widgets/WBP_Inventory.WBP_Inventory_C" (`GameplayStatics.GetPlayerController` 0) self))
      (set `self.InventoryWindow` _returnvalue)
      (bind _aspcont (cast `/Game/Blueprints/TemporalCharacter/PCont` (`GameplayStatics.GetPlayerController` 0)))
      ;[1 0.8504 0.2327] Add inventory widget as child to the HUD canvas
      (bind _returnvalue_2 (`CanvasPanel.AddChildToCanvas` (`/Game/Blueprints/InventorySystem/Widgets/WBP_HUD.HUDCanvas` (`/Game/Blueprints/TemporalCharacter/PCont.HUDWidget` _aspcont)) _inventorywindow))
      (`CanvasPanelSlot.SetAutoSize` _returnvalue_2 true)
      (`CanvasPanelSlot.SetOffsets` _returnvalue_2 (make `Margin` 0.0))
      (`CanvasPanelSlot.SetAnchors` _returnvalue_2 (make `Anchors` (0.0 0.0) (1.0 1.0)))
      (`CanvasPanelSlot.SetPosition` _returnvalue_2 (`self.Position`))
      (`WidgetBlueprintLibrary.SetInputMode_GameAndUIEx` (`GameplayStatics.GetPlayerController` 0) _inventorywindow "LockAlways")
      (`CharacterMovementComponent.DisableMovement` (`Character.CharacterMovement` (`GameplayStatics.GetPlayerCharacter` 0))))))