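; Spawner that creates NPC actors on demand through its SpawnActor event and registers them in the GameInstance's SpawnedNPCs array at ID minus one.
; Introduction spawns land at a random XY inside its Box at a fixed height.
; Other spawns use the given position, with radius zeroed and talking and moving flags set.
; The SetNPC helper applies name, skeletal mesh, ID and conversation ID to each new NPC.
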(event `SpawnActor`
  (params (Name :type Text) (Mesh :type "SkeletalMesh Object Reference") (ID :type Integer) (Position :type "Vector Structure") (ConversationID :type Integer) (Introduction :type Boolean))
  (bind _returnvalue (`GameplayStatics.GetGameInstance`))
  (bind _box (`self.Box`))
  (bind (_returnvalue_x _returnvalue_y) (`KismetMathLibrary.BreakVector` (`KismetMathLibrary.RandomPointInBoundingBox` (`SceneComponent.K2_GetComponentLocation` _box) (`BoxComponent.BoxExtent` _box))))
  (if Introduction
    (bind _returnvalue_2 (`|SpawnActorFromClass` "/Game/Blueprints/AI/NPC.NPC_C" (`KismetMathLibrary.MakeTransform` (`KismetMathLibrary.MakeVector` _returnvalue_x _returnvalue_y 120.0)) "Undefined" "OverrideRootScale" null null))
    (bind _spawnednpc (`self.SetNPC` _returnvalue_2 Name Mesh ID ConversationID))
    (bind _asgame_instance (cast `/Game/Blueprints/GameInstance` _returnvalue))
    (`KismetArrayLibrary.Array_Set` (`/Game/Blueprints/GameInstance.SpawnedNPCs` _asgame_instance) (- ID 1) _spawnednpc)
    (else
      (bind _returnvalue_3 (`|SpawnActorFromClass` "/Game/Blueprints/AI/NPC.NPC_C" (`KismetMathLibrary.MakeTransform` Position) "Undefined" "OverrideRootScale" null null))
      (bind _spawnednpc_2 (`self.SetNPC` _returnvalue_3 Name Mesh ID ConversationID))
      (set `/Game/Blueprints/AI/NPC.Radius` 0.0 _spawnednpc_2)
      (set `/Game/Blueprints/AI/NPC.IsTalking?` true _spawnednpc_2)
      (set `/Game/Blueprints/AI/NPC.IsMoving?` true _spawnednpc_2)
      (bind _asgame_instance_2 (cast `/Game/Blueprints/GameInstance` _returnvalue))
      (`KismetArrayLibrary.Array_Set` (`/Game/Blueprints/GameInstance.SpawnedNPCs` _asgame_instance_2) (- ID 1) _spawnednpc_2))))

(fn `SetNPC`
  (params (Ref :type "/Game/Blueprints/AI/NPC Object Reference") (Name :type Text) (Mesh :type "SkeletalMesh Object Reference") (ID :type Integer) (ConversationID :type Integer))
  (returns (SpawnedNPC :type "/Game/Blueprints/AI/NPC Object Reference"))
  (set `/Game/Blueprints/AI/NPC.CharacterName` Name Ref)
  (`SkinnedMeshComponent.SetSkinnedAssetAndUpdate` (`Character.Mesh` Ref) Mesh true)
  (set `/Game/Blueprints/AI/NPC.NPC_ID` ID Ref)
  (set `/Game/Blueprints/AI/NPC.Conversation_ID` ConversationID Ref)
  (return Ref))

(fn `UserConstructionScript`)