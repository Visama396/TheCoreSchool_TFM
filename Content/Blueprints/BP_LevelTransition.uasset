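; Stair transition actor that moves the player between the first floor, second floor and basement levels through overlap colliders.
; Each overlap walks the player character toward a set position while a fade-out level sequence plays with movement and look input disabled.
; When the sequence stops, SaveNextPlayerPosition opens the target level and stores the spawn position and rotation in GameInstanceTest for the next level.
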(event `self.RightStairsFirstFloor.OnComponentBeginOverlap`
  (params (OverlappedComponent :type "PrimitiveComponent Object Reference") (OtherActor :type "Actor Object Reference") (OtherComp :type "PrimitiveComponent Object Reference") (OtherBodyIndex :type Integer) (bFromSweep :type Boolean) (SweepResult :type "HitResult Structure (by ref)"))
  ;[0.2573 1 0.1697] Colliders First Floor: Move character to position while the sequence is playing. When the sequence is done, the player is teleported to the second floor
  (`self.MoveCharacter` (`self.PositionFirstFloorMoveToRightStairs`))
  (bind (_outactor _returnvalue) (`LevelSequencePlayer.CreateLevelSequencePlayer` "/Game/Sequences/S_ChangeLevelFadeOut.S_ChangeLevelFadeOut" (make `MovieSceneSequencePlaybackSettings` false (struct) 1.0 0.0 false false true true)))
  (`MovieSceneSequencePlayer.Play` _returnvalue)
  (add `MovieSceneSequencePlayer.OnStop` _returnvalue (delegate `RightStairsToFirstFloor`)))

(event `RightStairsToFirstFloor`
  ;[0.2573 1 0.1697] Colliders First Floor: Move character to position while the sequence is playing. When the sequence is done, the player is teleported to the second floor
  (`self.SaveNextPlayerPosition` (`self.SecondFloorName`) (`self.PositionSpawnSecondFloorRightStairs`) (`self.RotationStairsSecondFloor`)))

(event `self.LeftStairsFirstFloor.OnComponentBeginOverlap`
  (params (OverlappedComponent :type "PrimitiveComponent Object Reference") (OtherActor :type "Actor Object Reference") (OtherComp :type "PrimitiveComponent Object Reference") (OtherBodyIndex :type Integer) (bFromSweep :type Boolean) (SweepResult :type "HitResult Structure (by ref)"))
  ;[0.2573 1 0.1697] Colliders First Floor: Move character to position while the sequence is playing. When the sequence is done, the player is teleported to the second floor
  (`self.MoveCharacter` (`self.PositionFirstFloorMoveToLeftStairs`))
  (bind (_outactor _returnvalue) (`LevelSequencePlayer.CreateLevelSequencePlayer` "/Game/Sequences/S_ChangeLevelFadeOut.S_ChangeLevelFadeOut" (make `MovieSceneSequencePlaybackSettings` false (struct) 1.0 0.0 false false true true)))
  (`MovieSceneSequencePlayer.Play` _returnvalue)
  (add `MovieSceneSequencePlayer.OnStop` _returnvalue (delegate `LeftStairsToFirstFloor`)))

(event `LeftStairsToFirstFloor`
  ;[0.2573 1 0.1697] Colliders First Floor: Move character to position while the sequence is playing. When the sequence is done, the player is teleported to the second floor
  (`self.SaveNextPlayerPosition` (`self.SecondFloorName`) (`self.PositionSpawnSecondFloorLeftStairs`) (`self.RotationStairsSecondFloor`)))

(event `self.RightStairsSecondFloor.OnComponentBeginOverlap`
  (params (OverlappedComponent :type "PrimitiveComponent Object Reference") (OtherActor :type "Actor Object Reference") (OtherComp :type "PrimitiveComponent Object Reference") (OtherBodyIndex :type Integer) (bFromSweep :type Boolean) (SweepResult :type "HitResult Structure (by ref)"))
  ;[0.2425 0.2615 1] Colliders First Floor
  (`self.MoveCharacter` (`self.PositionSecondFloorMoveToRightStairs`))
  (bind (_outactor _returnvalue) (`LevelSequencePlayer.CreateLevelSequencePlayer` "/Game/Sequences/S_ChangeLevelFadeOut.S_ChangeLevelFadeOut" (make `MovieSceneSequencePlaybackSettings` false (struct) 1.0 0.0 false false true true)))
  (`MovieSceneSequencePlayer.Play` _returnvalue)
  (add `MovieSceneSequencePlayer.OnStop` _returnvalue (delegate `RightStairsToSecondFloor`)))

(event `RightStairsToSecondFloor`
  ;[0.2425 0.2615 1] Colliders First Floor
  (`self.SaveNextPlayerPosition` (`self.FirstFloorName`) (`self.PositionSpawnFirstFloorRightStairs`) (`self.RotationStairsFirstFloor`)))

(event `self.LeftStairsSecondFloor.OnComponentBeginOverlap`
  (params (OverlappedComponent :type "PrimitiveComponent Object Reference") (OtherActor :type "Actor Object Reference") (OtherComp :type "PrimitiveComponent Object Reference") (OtherBodyIndex :type Integer) (bFromSweep :type Boolean) (SweepResult :type "HitResult Structure (by ref)"))
  ;[0.2425 0.2615 1] Colliders First Floor
  (`self.MoveCharacter` (`self.PositionSecondFloorMoveToLeftStairs`))
  (bind (_outactor _returnvalue) (`LevelSequencePlayer.CreateLevelSequencePlayer` "/Game/Sequences/S_ChangeLevelFadeOut.S_ChangeLevelFadeOut" (make `MovieSceneSequencePlaybackSettings` false (struct) 1.0 0.0 false false true true)))
  (`MovieSceneSequencePlayer.Play` _returnvalue)
  (add `MovieSceneSequencePlayer.OnStop` _returnvalue (delegate `LeftStairsToSecondFloor`)))

(event `LeftStairsToSecondFloor`
  ;[0.2425 0.2615 1] Colliders First Floor
  (`self.SaveNextPlayerPosition` (`self.FirstFloorName`) (`self.PositionSpawnFirstFloorLeftStairs`) (`self.RotationStairsFirstFloor`)))

(event `self.StairsToBasement.OnComponentBeginOverlap`
  (params (OverlappedComponent :type "PrimitiveComponent Object Reference") (OtherActor :type "Actor Object Reference") (OtherComp :type "PrimitiveComponent Object Reference") (OtherBodyIndex :type Integer) (bFromSweep :type Boolean) (SweepResult :type "HitResult Structure (by ref)"))
  ;[1 0.2898 0.3395] Transition between Basement and first floor
  (`self.MoveCharacter` (`self.PositionFirstFloorMoveToBasement`))
  (bind (_outactor _returnvalue) (`LevelSequencePlayer.CreateLevelSequencePlayer` "/Game/Sequences/S_ChangeLevelFadeOut.S_ChangeLevelFadeOut" (make `MovieSceneSequencePlaybackSettings` false (struct) 1.0 0.0 false false true true)))
  (`MovieSceneSequencePlayer.Play` _returnvalue)
  (add `MovieSceneSequencePlayer.OnStop` _returnvalue (delegate `GoToBasement`)))

(event `GoToBasement`
  ;[1 0.2898 0.3395] Transition between Basement and first floor
  (`self.SaveNextPlayerPosition` (`self.BasementName`) (`self.PositionSpawnBasement`) (`self.RotationBasement`)))

(event `self.StairsFromBasement.OnComponentBeginOverlap`
  (params (OverlappedComponent :type "PrimitiveComponent Object Reference") (OtherActor :type "Actor Object Reference") (OtherComp :type "PrimitiveComponent Object Reference") (OtherBodyIndex :type Integer) (bFromSweep :type Boolean) (SweepResult :type "HitResult Structure (by ref)"))
  ;[1 0.2898 0.3395] Transition between Basement and first floor
  (`self.MoveCharacter` (`self.PositionBasementMove`))
  (bind (_outactor _returnvalue) (`LevelSequencePlayer.CreateLevelSequencePlayer` "/Game/Sequences/S_ChangeLevelFadeOut.S_ChangeLevelFadeOut" (make `MovieSceneSequencePlaybackSettings` false (struct) 1.0 0.0 false false true true)))
  (`MovieSceneSequencePlayer.Play` _returnvalue)
  (add `MovieSceneSequencePlayer.OnStop` _returnvalue (delegate `GoFirstFloorFromBasement`)))

(event `GoFirstFloorFromBasement`
  ;[1 0.2898 0.3395] Transition between Basement and first floor
  (`self.SaveNextPlayerPosition` (`self.FirstFloorName`) (`self.PositionSpawnFirstFloorFromBasement`) (`self.RotationStairsFirstFloor`)))

(fn `MoveCharacter`
  (params (Position :type "Vector Structure"))
  (bind _asplayer_character (cast `/Game/Blueprints/PlayerController/PlayerCharacter` (`GameplayStatics.GetPlayerCharacter` 0)))
  (`/Game/Blueprints/PlayerController/PlayerCharacter.MoveUsingStairs` _asplayer_character Position))

(fn `SaveNextPlayerPosition`
  (params (LevelName :type Name) (PlayerPosition :type "Vector Structure") (PlayerRotation :type "Rotator Structure"))
  ;[0.2358 0.1941 1] Saves the position of the player in the game Instance for the next level
  (`GameplayStatics.OpenLevel` LevelName)
  (bind _asgame_instance_test (cast `/Game/Blueprints/TemporalCharacter/GameInstanceTest` (`GameplayStatics.GetGameInstance`)))
  (`/Game/Blueprints/TemporalCharacter/GameInstanceTest.SetCharacterInitialPositionAndRotation` _asgame_instance_test PlayerPosition PlayerRotation))

(fn `UserConstructionScript`)