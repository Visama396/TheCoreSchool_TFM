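; Security keypad puzzle that opens a linked door when the player clicks in the correct code.
; Interaction blends the view to the panel, showing the cursor and hiding the player mesh.
; Single-use digit buttons append to an integer via strings, checked at the code's length; failure lights red and resets.
; Success lights green, restores the player view and rotates the door both instantly and by timeline; the reset button leaves entered digits intact.
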(event `/Game/Blueprints/BI_Interaction.Interaction`
  (params (Actor :type "Actor Object Reference"))
  (bind _returnvalue (`GameplayStatics.GetPlayerController` 0))
  ;[0.9291 0.3051 1] Change to the panel camera and hide player
  (`PlayerController.SetViewTargetWithBlend` _returnvalue self 2.0 "VTBlend_Linear" 1.0 false)
  (set `PlayerController.bShowMouseCursor` true _returnvalue)
  (`SceneComponent.SetVisibility` (`Character.Mesh` (`GameplayStatics.GetPlayerCharacter` 0)) false false))

(event `self.securityKeypad_Button__1_.OnClicked`
  (params (TouchedComponent :type "PrimitiveComponent Object Reference") (ButtonPressed :type "Key Structure"))
  ;[0.3047 1 0.9002] Buttons pressed
  (if (not (`self.1Pressed`))
    (set `self.1Pressed` true)
    (`self.PressButton` TouchedComponent 1)
    (if (`self.CodeIsCorrect?`) :!label _label
      (`KismetSystemLibrary.Delay` 1.0)
      (`self.BackToPlayerCameraAndOpenDoor`)
      (bind (_direction _doorrotation) (`Timeline|Timeline_0`)
        (:`Update`
          (`self.K2_SetActorRelativeRotation` (`self.DoorToOpen`) (`KismetMathLibrary.MakeRotator` 0.0 0.0 _doorrotation) false false))))))

(event `self.securityKeypad_Button__2_.OnClicked`
  (params (TouchedComponent :type "PrimitiveComponent Object Reference") (ButtonPressed :type "Key Structure"))
  ;[0.3047 1 0.9002] Buttons pressed
  (if (not (`self.2Pressed`))
    (set `self.2Pressed` true)
    (`self.PressButton` TouchedComponent 2)
    (goto _label)))

(event `self.securityKeypad_Button__3_.OnClicked`
  (params (TouchedComponent :type "PrimitiveComponent Object Reference") (ButtonPressed :type "Key Structure"))
  ;[0.3047 1 0.9002] Buttons pressed
  (if (not (`self.3Pressed`))
    (set `self.3Pressed` true)
    (`self.PressButton` TouchedComponent 3)
    (goto _label)))

(event `self.securityKeypad_Button__4_.OnClicked`
  (params (TouchedComponent :type "PrimitiveComponent Object Reference") (ButtonPressed :type "Key Structure"))
  ;[0.3047 1 0.9002] Buttons pressed
  (if (not (`self.4Pressed`))
    (set `self.4Pressed` true)
    (`self.PressButton` TouchedComponent 4)
    (goto _label)))

(event `self.securityKeypad_Button__5_.OnClicked`
  (params (TouchedComponent :type "PrimitiveComponent Object Reference") (ButtonPressed :type "Key Structure"))
  ;[0.3047 1 0.9002] Buttons pressed
  (if (not (`self.5Pressed`))
    (set `self.5Pressed` true)
    (`self.PressButton` TouchedComponent 5)
    (goto _label)))

(event `self.securityKeypad_Button__6_.OnClicked`
  (params (TouchedComponent :type "PrimitiveComponent Object Reference") (ButtonPressed :type "Key Structure"))
  ;[0.3047 1 0.9002] Buttons pressed
  (if (not (`self.6Pressed`))
    (set `self.6Pressed` true)
    (`self.PressButton` TouchedComponent 6)
    (goto _label)))

(event `self.securityKeypad_Button__7_.OnClicked`
  (params (TouchedComponent :type "PrimitiveComponent Object Reference") (ButtonPressed :type "Key Structure"))
  ;[0.3047 1 0.9002] Buttons pressed
  (if (not (`self.7Pressed`))
    (set `self.7Pressed` true)
    (`self.PressButton` TouchedComponent 7)
    (goto _label)))

(event `self.securityKeypad_Button__8_.OnClicked`
  (params (TouchedComponent :type "PrimitiveComponent Object Reference") (ButtonPressed :type "Key Structure"))
  ;[0.3047 1 0.9002] Buttons pressed
  (if (not (`self.8Pressed`))
    (set `self.8Pressed` true)
    (`self.PressButton` TouchedComponent 8)
    (goto _label)))

(event `self.securityKeypad_Button__9_.OnClicked`
  (params (TouchedComponent :type "PrimitiveComponent Object Reference") (ButtonPressed :type "Key Structure"))
  ;[0.3047 1 0.9002] Buttons pressed
  (if (not (`self.9Pressed`))
    (set `self.9Pressed` true)
    (`self.PressButton` TouchedComponent 9)
    (goto _label)))

(event `self.securityKeypad_Button__0_.OnClicked`
  (params (TouchedComponent :type "PrimitiveComponent Object Reference") (ButtonPressed :type "Key Structure"))
  ;[0.3047 1 0.9002] Buttons pressed
  (if (not (`self.0Pressed`))
    (set `self.0Pressed` true)
    (`self.PressButton` TouchedComponent)
    (goto _label)))

(event `self.securityKeypad_Button.OnClicked`
  (params (TouchedComponent :type "PrimitiveComponent Object Reference") (ButtonPressed :type "Key Structure"))
  ;[0.3047 1 0.9002] Buttons pressed
  (`self.ResetAllButtons`))

(fn `BackToPlayerCameraAndOpenDoor`
  ;[0.2944 0.3074 1] Return camera back to the player and hide mouse
  (`PlayerController.SetViewTargetWithBlend` (`GameplayStatics.GetPlayerController` 0) (`GameplayStatics.GetPlayerCharacter` 0) 2.0 "VTBlend_Linear" 1.0 false)
  (`SceneComponent.SetVisibility` (`Character.Mesh` (`GameplayStatics.GetPlayerCharacter` 0)) true false)
  (set `PlayerController.bShowMouseCursor` false (`GameplayStatics.GetPlayerController` 0))
  (`self.K2_AddActorLocalRotation` (`self.DoorToOpen`) (struct :`Yaw` 95.0) false false))

(fn `CheckCodeIntroduced`
  (params (NumberPressed :type Integer))
  ;[0.9987 1 0.1227] If the code is -1, it means no number was introduced
  (if (== (`self.CodeIntroduced`) -1)
    (set `self.CodeIntroduced` NumberPressed)
    (else
      ;[1 0.3987 0.5394] Append the code introduced until now with the new number
      (set `self.CodeIntroduced` (`KismetStringLibrary.Conv_StringToInt` (`KismetStringLibrary.Concat_StrStr` (`KismetStringLibrary.Conv_IntToString` (`self.CodeIntroduced`)) (`KismetStringLibrary.Conv_IntToString` NumberPressed))))
      ;[0.2816 0.7982 1] If the code introduced and the final code have the same length, compare them
      (if (== (`KismetStringLibrary.Len` (`KismetStringLibrary.Conv_IntToString` (`self.CorrectCode`))) (`KismetStringLibrary.Len` (`KismetStringLibrary.Conv_IntToString` (`self.CodeIntroduced`))))
        ;[0.6902 0.3008 1] If the code is correct turn on the green light, if not turn on the red light and reset the buttons
        (if (== (`self.CorrectCode`) (`self.CodeIntroduced`))
          (`PrimitiveComponent.SetMaterial` (`self.securityKeypad_LED_Green`) 0 "/Game/Models/Props/SecurityKeypad/LED_Green_On.LED_Green_On")
          (set `self.PressButtonPossible?` false)
          (set `self.CodeIsCorrect?` true)
          (else
            (`PrimitiveComponent.SetMaterial` (`self.securityKeypad_LED_Red`) 0 "/Game/Models/Props/SecurityKeypad/LED_Red_On.LED_Red_On")
            (set `self.CodeIntroduced` -1)
            (`self.ResetAllButtons`)))))))

(fn `PressButton`
  (params (ButtonPressed :type "PrimitiveComponent Object Reference") (Number :type Integer))
  ;[0.2655 1 0.1643] If button can be pressed, set the material, position and check code introduced
  (if (`self.PressButtonPossible?`)
    (`PrimitiveComponent.SetMaterial` (`self.securityKeypad_LED_Red`) 0 "/Game/Models/Props/SecurityKeypad/LED_Red.LED_Red")
    (`PrimitiveComponent.SetMaterial` ButtonPressed 0 "/Game/Models/Props/SecurityKeypad/Keypad_Buttons_Pressed_Inst.Keypad_Buttons_Pressed_Inst")
    (`SceneComponent.K2_SetWorldLocation` ButtonPressed (+ (`SceneComponent.K2_GetComponentLocation` ButtonPressed) (0.5 0.0 0.0)) false false)
    (`self.CheckCodeIntroduced` Number)))

(fn `ResetAllButtons`
  ;[0.1303 0.1921 1] Reset all the buttons and set the buttons bools to false
  (for _array_element (`SceneComponent.GetChildrenComponents` (`self.Buttons`) false)
    (bind _asstatic_mesh_component (cast `StaticMeshComponent` _array_element))
    (`self.ResetButtonBack` _asstatic_mesh_component)
    (set `self.1Pressed` false)
    (set `self.2Pressed` false)
    (set `self.3Pressed` false)
    (set `self.4Pressed` false)
    (set `self.5Pressed` false)
    (set `self.6Pressed` false)
    (set `self.7Pressed` false)
    (set `self.8Pressed` false)
    (set `self.9Pressed` false)
    (set `self.0Pressed` false)))

(fn `ResetButtonBack`
  (params (Button :type "StaticMeshComponent Object Reference"))
  ;[1 0.2611 0.1112] Reset material and location
  (`PrimitiveComponent.SetMaterial` Button 0 "/Game/Models/Props/SecurityKeypad/Keypad.Keypad")
  (`SceneComponent.K2_SetRelativeLocation` Button (0.0 0.0 0.0) false false))

(fn `UserConstructionScript`)