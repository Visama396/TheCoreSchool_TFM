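; BP_LightManagment is a trigger Blueprint that switches a set of referenced lights on and off as something enters or leaves its collision volume.
; On BeginPlay it applies the TurnOnLightBeginning flag, then begin and end overlap on CollisionComponent turn the lights on and off.
; ToggleLight loops over the Lights array and sets each PointLightComponent's visibility, with no filtering of the overlapping actor.
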(event `self.ReceiveBeginPlay`
  (`self.ToggleLight` (`self.TurnOnLightBeginning`)))

(event `self.CollisionComponent.OnComponentBeginOverlap`
  (params (OverlappedComponent :type "PrimitiveComponent Object Reference") (OtherActor :type "Actor Object Reference") (OtherComp :type "PrimitiveComponent Object Reference") (OtherBodyIndex :type Integer) (bFromSweep :type Boolean) (SweepResult :type "HitResult Structure (by ref)"))
  (`self.ToggleLight` true))

(event `self.CollisionComponent.OnComponentEndOverlap`
  (params (OverlappedComponent :type "PrimitiveComponent Object Reference") (OtherActor :type "Actor Object Reference") (OtherComp :type "PrimitiveComponent Object Reference") (OtherBodyIndex :type Integer))
  (`self.ToggleLight` false))

(fn `ToggleLight`
  (params (`TurnOn?` :type Boolean))
  (for _array_element (`self.Lights`)
    (`SceneComponent.SetVisibility` (`PointLight.PointLightComponent` _array_element) `TurnOn?` false)))

(fn `UserConstructionScript`)