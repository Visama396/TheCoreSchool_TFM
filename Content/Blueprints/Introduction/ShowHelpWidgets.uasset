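; Introduction actor that shows the player three tutorial help widgets in sequence: movement, camera rotation and interaction.
; The widgets are created on BeginPlay, then ShowHelpWidgets adds each in turn to the player controller's HUD widget.
; A chain of delays holds each one for a given time, hides it, waits briefly and removes it.
; Overlapping the Box component starts the sequence, marked as a test trigger.
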(event `self.ReceiveBeginPlay`
  ;[0.4076 1 0.2818] Initialize the variables for the help Widgets
  (bind _returnvalue (`|CreateWidget` "/Game/Blueprints/Introduction/Widgets/WBP_MovementHelp.WBP_MovementHelp_C"))
  (set `self.MovementHelpWidget` _returnvalue)
  (bind _returnvalue_2 (`|CreateWidget` "/Game/Blueprints/Introduction/Widgets/WBP_RotateCameraHelp.WBP_RotateCameraHelp_C"))
  (set `self.RotateHelpWidget` _returnvalue_2)
  (bind _returnvalue_3 (`|CreateWidget` "/Game/Blueprints/Introduction/Widgets/WBP_InteractionHelp.WBP_InteractionHelp_C"))
  (set `self.InteractionHelpWidget` _returnvalue_3))

(event `ShowHelpWidgets`
  (params (TimeBetweenWidgets :type "Float (double-precision)"))
  (bind _interactionhelpwidget (`self.InteractionHelpWidget`))
  (bind _movementhelpwidget (`self.MovementHelpWidget`))
  (bind _rotatehelpwidget (`self.RotateHelpWidget`))
  (bind _aspcont (cast `/Game/Blueprints/PlayerController/PCont` (`GameplayStatics.GetPlayerController` 0)))
  (bind _hudwidget (`/Game/Blueprints/PlayerController/PCont.HUDWidget` _aspcont))
  ;[0.2645 0.3567 1] Slide in and out all the help widgets and remove from parent afterwards
  (`/Game/Blueprints/InventorySystem/Widgets/WBP_HUD.AddHelpWidgetToHUD` _hudwidget (`self.MovementHelpWidget`))
  (`KismetSystemLibrary.Delay` TimeBetweenWidgets)
  (`/Game/Blueprints/Introduction/Widgets/WBP_MovementHelp.HideWidget` _movementhelpwidget)
  (`KismetSystemLibrary.Delay` 1.0)
  (`Widget.RemoveFromParent` _movementhelpwidget)
  (`/Game/Blueprints/InventorySystem/Widgets/WBP_HUD.AddHelpWidgetToHUD` _hudwidget (`self.RotateHelpWidget`))
  (`KismetSystemLibrary.Delay` TimeBetweenWidgets)
  (`/Game/Blueprints/Introduction/Widgets/WBP_RotateCameraHelp.HideWidget` _rotatehelpwidget)
  (`KismetSystemLibrary.Delay` 1.0)
  (`Widget.RemoveFromParent` _rotatehelpwidget)
  (`/Game/Blueprints/InventorySystem/Widgets/WBP_HUD.AddHelpWidgetToHUD` _hudwidget (`self.InteractionHelpWidget`))
  (`KismetSystemLibrary.Delay` TimeBetweenWidgets)
  (`/Game/Blueprints/Introduction/Widgets/WBP_InteractionHelp.HideWidget` _interactionhelpwidget)
  (`KismetSystemLibrary.Delay` 1.0)
  (`Widget.RemoveFromParent` _interactionhelpwidget))

(event `self.Box.OnComponentBeginOverlap`
  (params (OverlappedComponent :type "PrimitiveComponent Object Reference") (OtherActor :type "Actor Object Reference") (OtherComp :type "PrimitiveComponent Object Reference") (OtherBodyIndex :type Integer) (bFromSweep :type Boolean) (SweepResult :type "HitResult Structure (by ref)"))
  ;[1 1 1] Just a test
  (`self.ShowHelpWidgets` 5.0))

(fn `UserConstructionScript`)