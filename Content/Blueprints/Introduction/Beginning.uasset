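; Introduction Blueprint meant to script the game's opening, though its StartBeginning event is empty and the sequence is disconnected, so it never runs.
; The unwired chain disables the player's CanMove flag, lowers walk speed and flags the first spawned NPC from GameInstance as talking with zero radius.
; It then auto-walks the player to that NPC with SimpleMoveToActor and triggers its Interaction twice, timed by fixed delays.
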(event `Start Beginning`)

(fn `UserConstructionScript`)