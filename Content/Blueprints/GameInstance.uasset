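; Game instance that carries the player's spawn position, rotation and inventory across level transitions.
; One function stores the given position and rotation, then triggers an inventory save.
; The save clears the stored list and copies entries from the player character's ACInventory component, skipping placeholder slots named "Nothing".
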(fn `SaveInventory`
  ;[0.3126 1 0.1953] Save all the objects of the inventory in the game instance
  (bind _asplayer_character (cast `/Game/Blueprints/PlayerController/PlayerCharacter` (`GameplayStatics.GetPlayerCharacter` 0)))
  (`KismetArrayLibrary.Array_Clear` (`self.Inventory`))
  (for _array_element (`/Game/Blueprints/InventorySystem/PickableObjects/AC_Inventory.Inventory` (`/Game/Blueprints/PlayerController/PlayerCharacter.AC_Inventory` _asplayer_character))
    (if (`KismetTextLibrary.NotEqual_TextText` (`.Name_2_B3B5A6A145432A9B2505B5AE2F9FFDB6` (break `/Game/Blueprints/InventorySystem/PickableObjects/F_Object` (`.ObjectStructure_2_89C0947C4FA810AB2C118F9E115F387F` (break `/Game/Blueprints/InventorySystem/PickableObjects/F_Slot` _array_element)))) (`|FormatText` "Nothing"))
      (`KismetArrayLibrary.Array_Add` (`self.Inventory`) _array_element))))

(fn `Set Character Initial Pos Rot And Save Inventory`
  (params (CharacterPosition :type "Vector Structure") (CharacterRotation :type "Rotator Structure"))
  ;[0.3718 1 0.3431] The position and rotation are saved here, because this blueprint persist between level transition
  (set `self.CharacterInitialPosition` CharacterPosition)
  (set `self.CharacterInitialRotation` CharacterRotation)
  (`self.SaveInventory`))