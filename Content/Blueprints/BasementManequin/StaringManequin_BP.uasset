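; Basement mannequin actor that animates or freezes according to which way the player faces.
; Every tick, a dot product compares the player's forward vector with the mannequin's, ignoring position and line of sight.
; When they point the same general way, it restores time dilation and starts a looping Acknowledging animation.
; When they oppose, zero CustomTimeDilation freezes it and clears the flag, so the animation restarts next time.
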(event `self.ReceiveTick`
  (params (DeltaSeconds :type "Float (single-precision)"))
  ;[1 1 1] STARRING ANIMATION
  (if (>= (`KismetMathLibrary.Dot_VectorVector` (`SceneComponent.GetForwardVector` (`Actor.RootComponent` (`GameplayStatics.GetPlayerCharacter` 0))) (`SceneComponent.GetForwardVector` (`self.DefaultSceneRoot`))) 0.0)
    (if (not (`self.AnimationStarted`))
      (set `self.CustomTimeDilation` 1.0)
      (`SkeletalMeshComponent.PlayAnimation` (`self.SkeletalMesh`) "/Game/Models/Characters/Player/Acknowledging_Anim_mixamo_com.Acknowledging_Anim_mixamo_com" true)
      (set `self.AnimationStarted` true))
    (else
      (set `self.AnimationStarted` false)
      (set `self.CustomTimeDilation` 0.0))))

(fn `UserConstructionScript`
  (`parent.UserConstructionScript`))