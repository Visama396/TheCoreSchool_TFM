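; BP_Cameraman is an aquarium cameraman prop with body, hands and camera meshes and a camera bubble effect.
; On BeginPlay the HandMovements timeline rolls the hands between 60 and 0 degrees, and its event track activates the bubble particle component.
; The construction script applies the chosen material and pushes suit color, metalness and roughness to all three meshes.
; An emitter-spawn node for the bubbles is left unconnected.
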(event `self.ReceiveBeginPlay`
  (bind (_direction _rotation_alpha) (`Timeline|Hand Movements` :!via `PlayFromStart`)
    (:`Update`
      (`SceneComponent.K2_SetRelativeRotation` (`self.CM_Cameraman_Hands`) (`KismetMathLibrary.MakeRotator` (`KismetMathLibrary.Lerp` 60.0 0.0 _rotation_alpha)) false false))
    (:`Event`
      (`ActorComponent.Activate` (`self.P_CameraBubble`) true))))

(fn `UserConstructionScript`
  (bind _cm_cameraman (`self.CM_Cameraman`))
  (bind (_suit_color_r _suit_color_g _suit_color_b) (break `LinearColor` (`self.Suit Color`)))
  (bind _cm_cameraman_camera (`self.CM_Cameraman_Camera`))
  (`PrimitiveComponent.SetMaterial` _cm_cameraman 0 (`self.Cameraman Material`))
  (`PrimitiveComponent.SetMaterial` (`self.CM_Cameraman_Hands`) 0 (`self.Cameraman Material`))
  (`PrimitiveComponent.SetMaterial` _cm_cameraman_camera 0 (`self.Cameraman Material`))
  (`MeshComponent.SetVectorParameterValueOnMaterials` _cm_cameraman "Suit Color" (`KismetMathLibrary.MakeVector` _suit_color_r _suit_color_g _suit_color_b))
  (`MeshComponent.SetVectorParameterValueOnMaterials` (`self.CM_Cameraman_Hands`) "Suit Color" (`KismetMathLibrary.MakeVector` _suit_color_r _suit_color_g _suit_color_b))
  (`MeshComponent.SetVectorParameterValueOnMaterials` _cm_cameraman_camera "Suit Color" (`KismetMathLibrary.MakeVector` _suit_color_r _suit_color_g _suit_color_b))
  (`MeshComponent.SetScalarParameterValueOnMaterials` _cm_cameraman_camera "Metalness" (`self.Metalness`))
  (`MeshComponent.SetScalarParameterValueOnMaterials` (`self.CM_Cameraman_Hands`) "Metalness" (`self.Metalness`))
  (`MeshComponent.SetScalarParameterValueOnMaterials` _cm_cameraman "Metalness" (`self.Metalness`))
  (`MeshComponent.SetScalarParameterValueOnMaterials` _cm_cameraman_camera "Roughness" (`self.Roughness`))
  (`MeshComponent.SetScalarParameterValueOnMaterials` (`self.CM_Cameraman_Hands`) "Roughness" (`self.Roughness`))
  (`MeshComponent.SetScalarParameterValueOnMaterials` _cm_cameraman "Roughness" (`self.Roughness`)))