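; BP_WaterproofLight is a configurable waterproof light fixture for the Aquarium content, pairing a light mesh with two spot lights.
; The construction script applies the shared color, intensity and attenuation radius settings to both spot lights.
; It also creates a dynamic material instance on the mesh, setting its "Light Color" to color times intensity so the fixture matches the emitted light.
; The event graph holds no runtime logic.
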(fn `UserConstructionScript`
  (bind _spotlight1 (`self.SpotLight1`))
  (bind _light_color (`self.Light Color`))
  (bind _returnvalue (`PrimitiveComponent.CreateDynamicMaterialInstance` (`self.Waterproof_Light_Light`) 0 null))
  (`MaterialInstanceDynamic.SetVectorParameterValue` _returnvalue "Light Color" (* _light_color (`self.Light Intensity`)))
  (`LightComponent.SetLightColor` _spotlight1 _light_color true)
  (`LightComponent.SetLightColor` (`self.SpotLight`) _light_color true)
  (`PointLightComponent.SetAttenuationRadius` _spotlight1 (`self.Attenuation Radius`))
  (`PointLightComponent.SetAttenuationRadius` (`self.SpotLight`) (`self.Attenuation Radius`))
  (`LightComponent.SetIntensity` _spotlight1 (`self.Light Intensity`))
  (`LightComponent.SetIntensity` (`self.SpotLight`) (`self.Light Intensity`)))