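; Aquarium filter actor with a spline-shaped power wire, a plug and a bubble effect that can be toggled by the On variable.
; The construction script builds the wire from spline mesh components between consecutive spline points, then places the plug at the spline's end, yawed 180 degrees.
; PBubbles visibility follows On, applied both at construction and at BeginPlay.
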(event `self.ReceiveBeginPlay`
  (`SceneComponent.SetVisibility` (`self.P_Bubbles`) (`self.On`) false))

(fn `UserConstructionScript`
  (bind _spline (`self.Spline`))
  (bind _plug (`self.Plug`))
  (bind _returnvalue (`SplineComponent.GetNumberOfSplinePoints` _spline))
  (bind (_returnvalue_location _returnvalue_rotation) (`KismetMathLibrary.BreakTransform` (`SplineComponent.GetTransformAtSplinePoint` (`self.Spline`) _returnvalue "World" false)))
  (`|ExecutionSequence`
    (:`then_0`
      (`SceneComponent.SetVisibility` (`self.P_Bubbles`) (`self.On`) false))
    (:`then_1`
      (for _index (range (+ (- _returnvalue 2) 1))
        (bind _returnvalue_2 (`AddComponent|NODE_AddSplineMeshComponent-0` :`bManualAttachment` true))
        (`StaticMeshComponent.SetStaticMesh` _returnvalue_2 (`self.Wire Mesh`))
        (`SceneComponent.K2_AttachToComponent` _returnvalue_2 (`self.DefaultSceneRoot`) "None" "KeepRelative" "KeepRelative" "KeepRelative" true)
        (bind (_location _tangent) (`SplineComponent.GetLocationAndTangentAtSplinePoint` _spline _index "Local"))
        (bind (_location_2 _tangent_2) (`SplineComponent.GetLocationAndTangentAtSplinePoint` _spline (+ _index 1) "Local"))
        (`SplineMeshComponent.SetStartAndEnd` _returnvalue_2 _location _tangent _location_2 _tangent_2 true))
      (`SceneComponent.K2_SetWorldLocation` _plug _returnvalue_location false false)
      (`SceneComponent.K2_SetWorldRotation` _plug (`KismetMathLibrary.MakeRotator` (.roll _returnvalue_rotation) (.pitch _returnvalue_rotation) (+ (.yaw _returnvalue_rotation) 180.0)) false false))))