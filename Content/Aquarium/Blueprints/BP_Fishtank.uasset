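; BP_Fishtank is an aquarium tank actor with configurable waterproof lighting, set up entirely in its construction script.
; A dynamic instance of MI_Light is applied to the light fixture mesh, with its color set to light color times intensity.
; The same exposed color, intensity, attenuation radius and cone angles drive two spot lights, keeping fixture and lights in sync.
; The event graph contains no active logic.
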(fn `UserConstructionScript`
  (bind _light_color (`self.Light Color`))
  (bind _spotlight1 (`self.SpotLight1`))
  (bind _returnvalue (`KismetMaterialLibrary.CreateDynamicMaterialInstance` "/Game/Aquarium/Materials/Equipments/MI_Light.MI_Light"))
  (bind _output_get (set `self.Mat_Waterlight` _returnvalue))
  (`PrimitiveComponent.SetMaterial` (`self.Waterproof_Light_Light`) 0 _output_get)
  (`MaterialInstanceDynamic.SetVectorParameterValue` (`self.Mat_Waterlight`) "Light Color" (* _light_color (`self.Light Intensity`)))
  (`LightComponent.SetLightColor` _spotlight1 _light_color true)
  (`LightComponent.SetLightColor` (`self.SpotLight`) _light_color true)
  (`PointLightComponent.SetAttenuationRadius` _spotlight1 (`self.Attenuation Radius`))
  (`PointLightComponent.SetAttenuationRadius` (`self.SpotLight`) (`self.Attenuation Radius`))
  (`LightComponent.SetIntensity` _spotlight1 (`self.Light Intensity`))
  (`LightComponent.SetIntensity` (`self.SpotLight`) (`self.Light Intensity`))
  (`SpotLightComponent.SetInnerConeAngle` _spotlight1 (`self.Inner Cone Angle`))
  (`SpotLightComponent.SetInnerConeAngle` (`self.SpotLight`) (`self.Inner Cone Angle`))
  (`SpotLightComponent.SetOuterConeAngle` _spotlight1 (`self.Outter Cone Angle`))
  (`SpotLightComponent.SetOuterConeAngle` (`self.SpotLight`) (`self.Outter Cone Angle`)))