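; BP_Modern_Cupboard is a furniture Blueprint for a cupboard with a sliding door that opens and closes on interaction.
; The Interaction event uses a FlipFlop to alternately play or reverse the OpenDoor timeline, with a matching sound at the actor's location.
; The timeline lerps the door mesh along its relative X axis.
; An IsSliding flag blocks new interactions until the slide finishes.
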(event `/Game/Blueprints/BI_Interaction.Interaction`
  (params (Actor :type "Actor Object Reference"))
  (bind _returnvalue (`self.K2_GetActorLocation`))
  (if (not (`self.IsSliding?`))
    (`/Engine/EditorBlueprintResources/StandardMacros.FlipFlop`
      (:`A`
        (set `self.IsSliding?` true)
        (`GameplayStatics.PlaySoundAtLocation` "/Game/Sounds/Props_Sounds/SlideDoor_Open.SlideDoor_Open" _returnvalue (struct) 0.8 1.0 0.0 null null null)
        (bind (_direction _slideopen) (`Timeline|OpenDoor` :!label _label)
          (:`Update`
            (`SceneComponent.K2_SetRelativeLocation` (`self.SM_Cupboard_Sliding_Door`) (`KismetMathLibrary.MakeVector` (`KismetMathLibrary.Lerp` 0.0 -110.0 _slideopen)) false false))
          (:`Finished`
            (set `self.IsSliding?` (not (`self.IsSliding?`))))))
      (:`B`
        (set `self.IsSliding?` true)
        (`GameplayStatics.PlaySoundAtLocation` "/Game/Sounds/Props_Sounds/SlideDoor_Close.SlideDoor_Close" _returnvalue (struct) 0.8 1.0 0.0 null null null)
        (goto _label :!via `Reverse`)))))

(fn `UserConstructionScript`)