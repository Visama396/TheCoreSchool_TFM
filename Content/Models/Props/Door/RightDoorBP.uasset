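; RightDoorBP is a door prop that swings open and shut with sound as an actor enters and leaves its trigger.
; It records the first overlapping actor in WhoOpened, so only that actor's exit clears it and toggles the door again.
; If CanBeOpened is set, a shared FlipFlop alternates between the OpenDoor timeline and the reversed CloseDoor timeline, each interpolating the door's relative yaw.
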(event `self.Trigger.OnComponentBeginOverlap`
  (params (OverlappedComponent :type "PrimitiveComponent Object Reference") (OtherActor :type "Actor Object Reference") (OtherComp :type "PrimitiveComponent Object Reference") (OtherBodyIndex :type Integer) (bFromSweep :type Boolean) (SweepResult :type "HitResult Structure (by ref)"))
  (bind _door (`self.Door`))
  (bind _returnvalue (`SceneComponent.K2_GetComponentLocation` (`self.DefaultSceneRoot`)))
  (if (== (`self.WhoOpened`) null)
    (set `self.WhoOpened` OtherActor)
    (if (`self.CanBeOpened`) :!label _label
      (`/Engine/EditorBlueprintResources/StandardMacros.FlipFlop`
        (:`A`
          (`GameplayStatics.PlaySoundAtLocation` "/Game/Sounds/Props_Sounds/DoorOpen.DoorOpen" _returnvalue (struct) 0.5 1.0 0.0 "/Game/Sounds/Props_Sounds/DoorSoundAttenuation.DoorSoundAttenuation" null null)
          (bind (_direction _dooropen) (`Timeline|OpenDoor` :!via `PlayFromStart`)
            (:`Update`
              (`SceneComponent.K2_SetRelativeRotation` _door (`KismetMathLibrary.MakeRotator` 0.0 0.0 (`KismetMathLibrary.Lerp` (`self.DoorOpen`) (`self.DoorClose`) _dooropen)) false false))))
        (:`B`
          (`GameplayStatics.PlaySoundAtLocation` "/Game/Sounds/Props_Sounds/DoorShut.DoorShut" _returnvalue (struct) 0.5 1.0 0.0 "/Game/Sounds/Props_Sounds/DoorSoundAttenuation.DoorSoundAttenuation" null null)
          (bind (_direction_2 _closedoor) (`Timeline|CloseDoor` :!via `ReverseFromEnd`)
            (:`Update`
              (`SceneComponent.K2_SetRelativeRotation` _door (`KismetMathLibrary.MakeRotator` 0.0 0.0 (`KismetMathLibrary.Lerp` (`self.DoorOpen`) (`self.DoorClose`) _closedoor)) false false))))))))

(event `self.Trigger.OnComponentEndOverlap`
  (params (OverlappedComponent :type "PrimitiveComponent Object Reference") (OtherActor :type "Actor Object Reference") (OtherComp :type "PrimitiveComponent Object Reference") (OtherBodyIndex :type Integer))
  (if (== OtherActor (`self.WhoOpened`))
    (set `self.WhoOpened` null)
    (goto _label)))

(fn `UserConstructionScript`)